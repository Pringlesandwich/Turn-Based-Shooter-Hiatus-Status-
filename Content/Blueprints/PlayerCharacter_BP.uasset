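; First-person player character Blueprint that adds a directional dodge and creates the player UI widget on BeginPlay.
; Left Shift or gamepad right face button reads movement input, rotates it by capsule facing, and launches a velocity-change impulse with sound and left/right widget feedback.
; Ground friction and walk speed are briefly zeroed during the dodge, then restored before a delay re-enables it.
; Left mouse only plays a gun sound.
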(event `self.ReceiveBeginPlay`
  (bind _returnvalue (`|CreateWidget` "/Game/UI/PlayerCharacterUI.PlayerCharacterUI_C"))
  (bind _output_get (set `self.PlayerCharacterWidget` _returnvalue))
  (`UserWidget.AddToViewport` _output_get 0)
  (set `self.PlayerCamera` (`self.FirstPersonCameraComponent`)))

(event `self.ReceiveTick`
  (params (DeltaSeconds :type "Float (single-precision)")))

(event `Key|LeftShift`
  (params (Key :type "Key Structure" :default "AnyKey"))
  (bind _yinput (`self.YInput`))
  (bind _boostamount (`self.BoostAmount`))
  (bind _charactermovement (`self.CharacterMovement`))
  (bind _playercharacterwidget (`self.PlayerCharacterWidget`))
  (bind _charactermovement_2 (`self.CharacterMovement`))
  (bind (_returnvalue_x _returnvalue_y) (`KismetMathLibrary.BreakVector` (`KismetMathLibrary.GreaterGreater_VectorRotator` (`KismetMathLibrary.Conv_RotatorToVector` (`SceneComponent.K2_GetComponentRotation` (`self.CapsuleComponent`))) (`KismetMathLibrary.Conv_VectorToRotator` (`KismetMathLibrary.MakeVector` (`self.XInput`) _yinput)))))
  ;[1 1 1] Dodge
  (:`Pressed`
    (if (`self.CanDodge`) :!label _label
      (set `self.CanDodge` false)
      (bind (_moveforward _moveright) (`self.GetMovementInput`))
      (set `self.XInput` _moveforward)
      (set `self.YInput` _moveright)
      (if (not (and (== _moveforward 0.0) (== _moveright 0.0)))
        (set `MovementComponent.Velocity` (0.0 0.0 0.0) (`self.CharacterMovement`))
        (`|ExecutionSequence`
          (:`then_0`
            (if (> _yinput 0.0)
              (`/Game/UI/PlayerCharacterUI.DodgeRight` _playercharacterwidget)))
          (:`then_1`
            (if (< _yinput 0.0)
              (`/Game/UI/PlayerCharacterUI.DodgeLeft` _playercharacterwidget)))
          (:`then_2`
            ;[1 1 1] Remove for old method
            (set `CharacterMovementComponent.GroundFriction` 0.0 _charactermovement_2)
            (set `CharacterMovementComponent.MaxWalkSpeed` 0.0 _charactermovement_2)
            (`CharacterMovementComponent.AddImpulse` (`self.CharacterMovement`) (`KismetMathLibrary.MakeVector` (* _returnvalue_x _boostamount) (* _returnvalue_y _boostamount) 100.0) true)
            (`GameplayStatics.PlaySoundAtLocation` "/Game/Sound/DodgePrefab.DodgePrefab" (`SceneComponent.K2_GetComponentLocation` (`self.CapsuleComponent`)))
            (set `self.XInput` 0.0)
            (set `self.YInput` 0.0)
            (`KismetSystemLibrary.Delay` 0.2)
            ;[1 1 1] Remove for old method
            (set `CharacterMovementComponent.GroundFriction` 8.0 _charactermovement)
            (set `CharacterMovementComponent.MaxWalkSpeed` 600.0 _charactermovement)
            (`KismetSystemLibrary.Delay` 0.5)
            (set `self.CanDodge` true)))))))

(event `Key|Gamepad_FaceButton_Right`
  (params (Key :type "Key Structure" :default "AnyKey"))
  ;[1 1 1] Dodge
  (:`Pressed`
    (goto _label)))

(event `Key|LeftMouseButton`
  (params (Key :type "Key Structure" :default "AnyKey"))
  (:`Pressed`
    (`GameplayStatics.PlaySoundAtLocation` "/Game/Sound/GunPrefab.GunPrefab" (`SceneComponent.K2_GetComponentLocation` (`self.GunPlaceholder`)))))

(fn `UserConstructionScript`)