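; Test game mode that sets up local multiplayer and handles spawning and despawning of player pawns.
; BeginPlay caches all PlayerStart actors and creates local players in a counted loop.
; SpawnPlayer swaps an existing pawn for a possessed PlayerCharacter_BP, while DespawnPlayer spawns an InitPawn but leaves the Possess target unset.
; Both use random PlayerStart transforms and point the view at a shared GameCamera.
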(event `self.ReceiveBeginPlay`
  (bind _number_of_players (`self.Number Of Players`))
  ;[1 1 1] Spawn 2 FirstPersonControllers
  (bind _outactors (`GameplayStatics.GetAllActorsOfClass` "/Script/Engine.PlayerStart"))
  (set `self.SpawnPoints` _outactors)
  (while (<= _number_of_players 2)
    (set `self.Number Of Players` (+ _number_of_players 1))
    (`GameplayStatics.CreatePlayer` -1)))

(event `SpawnPlayer`
  (params (PlayerController :type "PlayerController Object Reference"))
  (bind _returnvalue (`Controller.K2_GetPawn` PlayerController))
  ;[1 1 1] Spawn Player - destroys pawn if one is there, then creates a FPController and posses it
  (`/Engine/EditorBlueprintResources/StandardMacros.IsValid` _returnvalue
    (:`Is Valid`
      (`self.K2_DestroyActor` _returnvalue)
      (bind _returnvalue_2 (`|SpawnActorFromClass` "/Game/Blueprints/PlayerCharacter_BP.PlayerCharacter_BP_C" (`self.GetRandomSpawn`) "Undefined" "OverrideRootScale"))
      (`Controller.Possess` PlayerController _returnvalue_2)
      (`PlayerController.SetViewTargetWithBlend` PlayerController (`self.GameCamera`) 0.0 "VTBlend_Linear" 0.0 false))))

(event `DespawnPlayer`
  (params (PlayerController :type "PlayerController Object Reference"))
  (bind _returnvalue (`Controller.K2_GetPawn` PlayerController))
  ;[1 1 1] Despawn Player
  (`/Engine/EditorBlueprintResources/StandardMacros.IsValid` _returnvalue
    (:`Is Valid`
      (`self.K2_DestroyActor` _returnvalue)
      (`|SpawnActorFromClass` "/Game/Blueprints/InitPawn.InitPawn_C" (`self.GetRandomSpawn`) "Undefined" "OverrideRootScale")
      (`Controller.Possess` PlayerController null)
      (`PlayerController.SetViewTargetWithBlend` PlayerController (`self.GameCamera`) 0.0 "VTBlend_Linear" 0.0 false))))

(fn `UserConstructionScript`)