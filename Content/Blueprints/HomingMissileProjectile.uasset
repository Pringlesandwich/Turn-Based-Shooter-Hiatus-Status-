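; HomingMissileProjectile is a missile Blueprint that destroys whatever actor it hits, then destroys itself.
; On Hit it stores the other actor, loops over all PlayerCharacter_BP actors re-assigning any match, and prints the actor's name before and after.
; The loop does not restrict destruction to players.
; GetTarget takes a target player but is empty, and the graphs contain no homing logic.
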(event `GetTarget`
  (params (TargetPlayer :type "PlayerCharacter Object Reference")))

(event `self.ReceiveHit`
  (params (MyComp :type "PrimitiveComponent Object Reference") (Other :type "Actor Object Reference") (OtherComp :type "PrimitiveComponent Object Reference") (bSelfMoved :type Boolean) (HitLocation :type "Vector Structure") (HitNormal :type "Vector Structure") (NormalImpulse :type "Vector Structure") (Hit :type "HitResult Structure (by ref)"))
  (bind _todestroy (`self.ToDestroy`))
  (bind _output_get (set `self.ToDestroy` Other))
  (`KismetSystemLibrary.PrintString` (`KismetSystemLibrary.GetDisplayName` _output_get))
  (bind _outactors (`GameplayStatics.GetAllActorsOfClass` "/Game/Blueprints/PlayerCharacter_BP.PlayerCharacter_BP_C"))
  (for _array_element _outactors
    (if (== _array_element (`self.ToDestroy`))
      (set `self.ToDestroy` _array_element)))
  (`KismetSystemLibrary.PrintString` (`KismetSystemLibrary.GetDisplayName` _todestroy))
  (`self.K2_DestroyActor` _todestroy)
  (`self.K2_DestroyActor`))

(fn `UserConstructionScript`)